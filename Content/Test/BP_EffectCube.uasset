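; Pickup cube that applies a Gameplay Effect to an overlapping Player-tagged actor whose configured attribute is below its max.
; It passes the magnitude via SetByCaller tag, then immediately removes active instances of that effect class.
; Collision turns off and a timeline shrinks the cube, restarting an emissive fade on each update.
; The fade drives a dynamic material and destroys the actor when finished.
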(event EventBeginPlay
  (bind _returnvalue (Rendering|Material|CreateDynamicMaterialInstance (Variables|Default|GetCube) 0 0 "None" :!class /Script/Engine.PrimitiveComponent))
  (Variables|Default|SetDynamicMI _returnvalue))

(event Collision|EventActorBeginOverlap
  (params (OtherActor :type Actor%20Object%20Reference))
  (bind _returnvalue (Ability|GetAbilitySystemComponent OtherActor))
  (Utilities|IsValid _returnvalue
    (:Is%20Valid
      (if (Actor|ActorHasTag OtherActor "Player")
        (if (< (.ReturnValue (Ability|Attribute|GetFloatAttributefromAbilitySystemComponent _returnvalue (Variables|Default|GetAttribute))) (.ReturnValue (Ability|Attribute|GetFloatAttributefromAbilitySystemComponent _returnvalue (Variables|Default|GetMaxAttribute))))
          (bind _returnvalue_2 (Spec|MakeSpecHandle(ByClass) (Variables|Default|GetGameplay%20Effect) 0 self))
          (bind _returnvalue_3 (Ability|GameplayEffect|AssignTagSetbyCallerMagnitude _returnvalue_2 (Variables|Default|GetData%20Tag) (Variables|Default|GetEffectMagnitude)))
          (GameplayEffects|ApplyGameplayEffectSpecToSelf _returnvalue _returnvalue_3)
          (GameplayEffects|RemoveActiveGameplayEffectbySourceEffect _returnvalue (Variables|Default|GetGameplay%20Effect) 0 -1)
          (Collision|SetCollisionEnabled (Variables|Default|GetBoxCollider) "NoCollision")
          (bind _scale (Timeline|Scale PlayFromStart)
            (:Update
              (Transformation|SetWorldScale3D (Variables|Default|GetCube) (Math|Conversions|ToVector(Float) (Math|Float|Lerp 1.0 0.0 _scale)))
              (bind _fade (Timeline|Fade PlayFromStart)
                (:Update
                  (Rendering|Material|SetScalarParameterValue (Variables|Default|GetDynamicMI) "Emmissive" (Math|Float|Lerp (Variables|Default|GetEmmissive) 0.0 _fade) :!class /Script/Engine.MaterialInstanceDynamic))
                (:Finished
                  (Actor|DestroyActor))))))))))

(event Collision|EventActorEndOverlap
  (params (OtherActor :type Actor%20Object%20Reference))
  (Utilities|IsValid (Ability|GetAbilitySystemComponent OtherActor)))

(fn ConstructionScript)
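; BP_SoulCube is a test pickup that modifies souls on an overlapping actor that has an Ability System Component.
; It applies GE_ModifySouls with SoulMagnitude as a Data.Souls SetByCaller value, then immediately calls removal of that effect by source effect.
; It then disables the box collider to prevent retriggering and plays a timeline that fades the cube's emissive material parameter to zero.
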(event EventBeginPlay)

(event Collision|EventActorBeginOverlap
  (params (OtherActor :type Actor%20Object%20Reference))
  (bind _returnvalue (Ability|GetAbilitySystemComponent OtherActor))
  (Utilities|IsValid _returnvalue
    (:Is%20Valid
      (bind _returnvalue_2 (Spec|MakeSpecHandle(ByClass) "/Game/GameplayAbilitySystem/Effects/GE_ModifySouls.GE_ModifySouls_C" 0 self))
      (bind _returnvalue_3 (Ability|GameplayEffect|AssignTagSetbyCallerMagnitude _returnvalue_2 "(TagName=\"Data.Souls\")" (Variables|Default|GetSoulMagnitude)))
      (GameplayEffects|ApplyGameplayEffectSpecToSelf _returnvalue _returnvalue_3)
      (GameplayEffects|RemoveActiveGameplayEffectbySourceEffect _returnvalue "/Game/GameplayAbilitySystem/Effects/GE_ModifySouls.GE_ModifySouls_C" 0 -1)
      (Collision|SetCollisionEnabled (Variables|Default|GetBoxCollider) "NoCollision")
      (bind _fade (Timeline|Timeline PlayFromStart)
        (:Update
          (Rendering|Material|SetScalarParameterValueonMaterials (Variables|Default|GetCube) "Emmissive" (Math|Float|Lerp 7.5 0.0 _fade)))))))

(event Collision|EventActorEndOverlap
  (params (OtherActor :type Actor%20Object%20Reference)))

(fn ConstructionScript)
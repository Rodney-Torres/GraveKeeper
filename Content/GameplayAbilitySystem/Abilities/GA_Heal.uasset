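; Lantern heal ability that ends at once at full health, otherwise commits its cost and plays a cast montage.
; A montage gameplay event adds the heal cue, applies an infinite heal-over-time effect with SetByCaller magnitude and starts a looping timer.
; The clamp event removes the effect once health gained since activation reaches the per-use cap.
; Montage completion or interruption ends the ability, clearing timer, cue and effect.
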(event Custom|ClampMaxHeals
  ;[0.15 0.15 0.15 0.5] Remove GE if player reaches max heals
  (if (>= (- (.ReturnValue (Ability|Attribute|GetFloatAttribute (Ability|GetAvatarActorfromActorInfo) "(AttributeName=\"Health\",Attribute=/Script/GK.GKBasicAttributeSet:Health,AttributeOwner=\"/Script/CoreUObject.Class'/Script/GK.GKBasicAttributeSet'\")")) (Variables|Default|GetHealthOnAbilityUse)) (Variables|Default|GetMaxHealPerUse))
    (Ability|RemoveGameplayEffectFromOwnerWithHandle (Variables|Default|GetGEHandle))))

(event Ability|EventActivateAbility
  (bind _returnvalue (Ability|GetAvatarActorfromActorInfo))
  (bind _returnvalue_2 (Ability|Attribute|GetFloatAttribute _returnvalue "(AttributeName=\"Health\",Attribute=/Script/GK.GKBasicAttributeSet:Health,AttributeOwner=\"/Script/CoreUObject.Class'/Script/GK.GKBasicAttributeSet'\")"))
  ;[0.15 0.15 0.15 0.5] Set Start Health and Check if Player has full Health
  (Variables|Default|SetHealthOnAbilityUse _returnvalue_2)
  (if (== _returnvalue_2 (.ReturnValue (Ability|Attribute|GetFloatAttribute _returnvalue "(AttributeName=\"MaxHealth\",Attribute=/Script/GK.GKBasicAttributeSet:MaxHealth,AttributeOwner=\"/Script/CoreUObject.Class'/Script/GK.GKBasicAttributeSet'\")")))
    (Ability|EndAbility)
    (Development|PrintString "Full Health")
    (else
      (Development|PrintString "Heal Started")
      (Ability|CommitAbilityCost false)
      (|PlayMontageandWaitProxy "None" "/Game/CombatMagicAnims/Animations/AM_UE_AS_CastSpell_Arms.AM_UE_AS_CastSpell_Arms" 1.0 "None" true 1.0 0.0 true
        (:then
          (Ability|Tasks|WaitGameplayEvent "(TagName=\"Event.Montage.Trigger.Heal\")" 0
            (:EventReceived
              (GameplayCue|AddGameplayCue :GameplayCueTag "(TagName=\"GameplayCue.Lantern.Heal\")")
              (bind _returnvalue_3 (Utilities|Time|SetTimerbyEvent (EventDispatchers|CreateEvent :!event Custom|ClampMaxHeals) 0.033333 true))
              (Variables|Default|SetTimerHandle _returnvalue_3)
              (bind _returnvalue_4 (Ability|GameplayEffect|AssignTagSetbyCallerMagnitude (Ability|MakeOutgoingGameplayEffectSpec "/Game/GameplayAbilitySystem/Effects/GE_Lantern_HealOverTime_Infinite.GE_Lantern_HealOverTime_Infinite_C") "(TagName=\"Data.Heal\")" (Variables|Default|GetHealMagnitude)))
              (bind _returnvalue_5 (Ability|ApplyGameplayEffectSpecToOwner _returnvalue_4))
              (Variables|Default|SetGEHandle _returnvalue_5))))
        (:OnCompleted
          (Ability|EndAbility :!label _label))
        (:OnInterrupted
          (goto _label))
        (:OnCancelled
          (goto _label))))))

(event Ability|EventOnEndAbility
  (params (bWasCancelled :type Boolean))
  (Development|PrintString "Heal Ended")
  (Utilities|Time|ClearandInvalidateTimerbyHandle (Variables|Default|GetTimerHandle))
  (GameplayCue|RemoveGameplayCue "(TagName=\"GameplayCue.Lantern.Heal\")")
  (Ability|RemoveGameplayEffectFromOwnerWithHandle (Variables|Default|GetGEHandle)))
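; Base gameplay ability for enemy ranged attacks, driving hit scans on the avatar's equipped weapon through montage-timed gameplay events.
; It gets the weapon from WeaponsManagerComponent, plays AttackMontage and ends when that finishes or is interrupted.
; HitScan start and end events toggle the weapon's scan, passing a set-by-caller damage effect spec.
; Children override empty MontageStarted and SetMontage hooks, the latter called when no montage is valid.
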(event Custom|MontageStarted
  ;[0.15 0.15 0.15 0.5] Does Nothing. Override in Child
)

(event Custom|HandleHitScanStart
  (bind _damagemagnitude (Variables|Stats|GetDamageMagnitude))
  ;[1 0 0 0.5] HitScan Events
  (bind _equipped_weapon (Variables|Default|GetEquipped%20Weapon)
    (:then
      (bind _returnvalue (Ability|GameplayEffect|AssignTagSetbyCallerMagnitude (Ability|MakeOutgoingGameplayEffectSpec (Variables|GameplayEffect|GetGameplay%20Effect%20Class)) "(TagName=\"Data.Damage\")" _damagemagnitude))
      (Default|StartHitScan _equipped_weapon _returnvalue)
      (Development|PrintString (Utilities|String|ToString(Float) _damagemagnitude)))
    (:else)))

(event Custom|HandleHitScanEnd
  ;[1 0 0 0.5] HitScan Events
  (bind _equipped_weapon (Variables|Default|GetEquipped%20Weapon)
    (:then
      (Default|EndHitScan _equipped_weapon))
    (:else)))

(event Custom|SetMontage
  ;[0.15 0.15 0.15 0.5] Does Nothing. Override in Child
)

(event Ability|EventActivateAbility
  (bind _returnvalue (Ability|GetAvatarActorfromActorInfo))
  (bind _returnvalue_2 (Actor|GetComponentbyClass _returnvalue "/Game/Weapons/WeaponsManagerComponent.WeaponsManagerComponent_C"))
  (Utilities|IsValid _returnvalue_2
    (:Is%20Valid
      (bind _equippedweapon (Variables|/Game/Weapons/WeaponsManagerComponent.WeaponsManagerComponent_C|GetEquippedWeapon _returnvalue_2)
        (:then
          (Variables|Default|SetEquipped%20Weapon _equippedweapon)
          (bind _attackmontage (Variables|Anim|GetAttackMontage)
            (:then
              (|PlayMontageandWaitProxy "None" _attackmontage 1.0 (Variables|Default|GetStart%20Section) true 1.0 0.0 true
                (:then
                  (CallFunction|MontageStarted)
                  (Ability|Tasks|WaitGameplayEvent "(TagName=\"Event.HitScan.Start\")" 0 :!label _label
                    (:then
                      (Ability|Tasks|WaitGameplayEvent "(TagName=\"Event.HitScan.End\")" 0
                        (:EventReceived
                          (CallFunction|HandleHitScanEnd))))
                    (:EventReceived
                      (CallFunction|HandleHitScanStart))))
                (:OnCompleted
                  (Ability|EndAbility :!label _label_2))
                (:OnInterrupted
                  (goto _label_2))
                (:OnCancelled
                  (goto _label_2))))
            (:else
              (CallFunction|SetMontage)
              (goto _label))))
        (:else
          (Ability|EndAbility :!label _label_3))))
    (:Is%20Not%20Valid
      (goto _label_3))))

(event Ability|EventOnEndAbility
  (params (bWasCancelled :type Boolean))
  (CallFunction|HandleHitScanEnd))
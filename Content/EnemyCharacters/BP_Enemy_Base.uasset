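; BP_Enemy_Base is the base zombie enemy character, providing combat, weapon and movement functions.
; Attack activates a melee ability through the GK ability system and signals its end on the next tick, without waiting for the ability to finish.
; Scream montages drive weapon spawning and deletion, with notifies triggering WeaponsManagerComponent changes and completion firing callbacks.
; Getter and setter functions supply combat ranges, a patrol route and speed-tier walk speeds.
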(event Custom|Attack
  (Abilities|TryActivateAbilitybyClass (Variables|Default|GetGKAbilitySystemComponent) "/Game/GameplayAbilitySystem/Abilities/GA_Zombie_MeleeAttack.GA_Zombie_MeleeAttack_C" true)
  (Utilities|FlowControl|DelayUntilNextTick)
  (Default|CallOnAttackEnd))

(event Custom|SpawnWeapon
  (bind _notifyname (Animation|Montage|PlayMontage (Variables|Character|GetMesh) "/Game/EnemyCharacters/Montages/AM_Zombie_Scream_SpawnWeapon.AM_Zombie_Scream_SpawnWeapon")
    (:OnCompleted
      (Default|CallOnSpawnWeapon))
    (:OnNotifyBegin
      (switch name _notifyname
        (:SpawnWeapon
          (Default|SpawnWeapon (Variables|Default|GetWeaponsManagerComponent) "/Game/EnemyCharacters/Weapons/BP_RightHand.BP_RightHand_C")
          (Variables|/Game/Weapons/WeaponsManagerComponent.WeaponsManagerComponent_C|GetEquippedWeapon (Variables|Default|GetWeaponsManagerComponent)
            (:then
              (Variables|Default|SetHasWeapon true))
            (:else)))))))

(event Custom|DeleteWeapon
  (bind _notifyname (Animation|Montage|PlayMontage (Variables|Character|GetMesh) "/Game/EnemyCharacters/Montages/AM_Zombie_Scream_DeleteWeapon.AM_Zombie_Scream_DeleteWeapon")
    (:OnCompleted
      (Default|CallOnDeleteWeapon))
    (:OnNotifyBegin
      (switch name _notifyname
        (:DeleteWeapon
          (Actor|DestroyActor (Variables|/Game/Weapons/WeaponsManagerComponent.WeaponsManagerComponent_C|GetEquippedWeapon (Variables|Default|GetWeaponsManagerComponent)))
          (Variables|Default|SetHasWeapon false))))))

(event EventBeginPlay)

(fn ConstructionScript)

(fn GetIdealRange
  (return 1.5e+02 3.5e+02))

(fn GetPatrolRoute
  (return (Variables|AI|GetPatrolRoute)))

(fn SetMovementSpeed
  (params (Speed :type E_MovementSpeed%20Enum :default "NewEnumerator0"))
  (bind _output_get (Variables|/Script/Engine.CharacterMovementComponent|SetMaxWalkSpeed (Variables|Character|GetCharacterMovement) (Utilities|Select :Index Speed :NewEnumerator0 0.0 :NewEnumerator1 2e+02 :NewEnumerator2 3e+02 :NewEnumerator3 4e+02)))
  (return _output_get))
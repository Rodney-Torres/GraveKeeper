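; BP_Zombie is a zombie enemy character that receives its melee attacks through the Gameplay Ability System.
; On BeginPlay it runs the parent logic, then GiveAbilities grants two melee abilities to its GKAbilitySystemComponent.
; Tick and the construction script only call the parent, and an unconnected node that would activate the second melee ability never runs.
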(event EventBeginPlay
  (|CallParentFunction)
  (CallFunction|GiveAbilities))

(event Collision|EventActorBeginOverlap
  (params (OtherActor :type Actor%20Object%20Reference))
  (|CallParentFunction OtherActor) ; This node is disabled and will not be called.\nDrag off pins to build functionality.
)

(event EventTick
  (params (DeltaSeconds :type Float%20%28single-precision%29))
  (|CallParentFunction DeltaSeconds))

(fn ConstructionScript
  (|CallParentFunction))

(fn GiveAbilities
  (GameplayAbilities|GiveAbility (Variables|Default|GetGKAbilitySystemComponent) "/Game/EnemyCharacters/Zombie/Abilities/GA_Zombie_Melee1.GA_Zombie_Melee1_C" 0 -1)
  (GameplayAbilities|GiveAbility (Variables|Default|GetGKAbilitySystemComponent) "/Game/EnemyCharacters/Zombie/Abilities/GA_Zombie_Melee2.GA_Zombie_Melee2_C" 0 -1))
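; BP_Enemy_Ranged is a ranged zombie enemy Blueprint that equips itself with a weapon when play begins.
; After the parent BeginPlay, SpawnWeapon has the WeaponsManagerComponent spawn the configured WeaponClass.
; A valid equipped weapon sets HasWeapon and fires CallOnWeaponSpawn.
; The Attack event is empty, and the construction script only calls its parent.
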(event EventBeginPlay
  (|CallParentFunction)
  (CallFunction|SpawnWeapon))

(event EventSpawnWeapon
  (Default|SpawnWeapon (Variables|Default|GetWeaponsManagerComponent) (Variables|Default|GetWeapon%20Class))
  (Variables|/Game/Weapons/WeaponsManagerComponent.WeaponsManagerComponent_C|GetEquippedWeapon (Variables|Default|GetWeaponsManagerComponent)
    (:then
      (Variables|Default|SetHasWeapon true)
      (Default|CallOnWeaponSpawn))
    (:else)))

(event EventAttack)

(fn ConstructionScript
  (|CallParentFunction))
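; Ranged zombie enemy Blueprint that spawns a weapon on BeginPlay and supplies its own attack and defend radii and movement speeds.
; Attack and aggro alert activate GAS abilities, though the attack currently uses the melee zombie ability.
; Completion callbacks are timed rather than ability-driven: attack end fires next tick, and alert end follows a fixed delay that the author notes as needing a montage-event fix.
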(event EventBeginPlay
  (|CallParentFunction)
  (CallFunction|SpawnWeapon))

(event EventAggroAlert
  (Abilities|TryActivateAbilitybyClass (Variables|Default|GetGKAbilitySystemComponent) "/Game/EnemyCharacters/Enemies/Zombie_Melee/GA/GA_Zombie_AggroAlert.GA_Zombie_AggroAlert_C" true)
  ;[0.15 0.15 0.15 0.5] To fix this I could put an event in the montage to trigger the calling/finish exectuting nodes.
  (Utilities|FlowControl|Delay 2.0)
  (Default|CallOnAggroAlertEnd))

(event EventSpawnWeapon
  (Default|SpawnWeapon (Variables|Default|GetWeaponsManagerComponent) (Variables|Default|GetWeapon%20Class))
  (Variables|/Game/Weapons/WeaponsManagerComponent.WeaponsManagerComponent_C|GetEquippedWeapon (Variables|Default|GetWeaponsManagerComponent)
    (:then
      (Variables|Default|SetHasWeapon true)
      (Default|CallOnWeaponSpawn))
    (:else)))

(event EventAttack
  (Abilities|TryActivateAbilitybyClass (Variables|Default|GetGKAbilitySystemComponent) "/Game/EnemyCharacters/Enemies/Zombie_Melee/GA/GA_Zombie_Melee_Attack1.GA_Zombie_Melee_Attack1_C" true)
  (Utilities|FlowControl|DelayUntilNextTick)
  (Default|CallOnAttackEnd))

(fn ConstructionScript
  (|CallParentFunction))

(fn GetIdealRange
  (return 2e+02 8e+02))

(fn SetMovementSpeed
  (params (Speed :type E_MovementSpeed%20Enum :default "NewEnumerator0"))
  (Variables|/Script/Engine.CharacterMovementComponent|SetMaxWalkSpeed (Variables|Character|GetCharacterMovement) (Utilities|Select :Index Speed :NewEnumerator0 0.0 :NewEnumerator1 1e+02 :NewEnumerator2 3e+02 :NewEnumerator3 4e+02))
  (return 0.0))
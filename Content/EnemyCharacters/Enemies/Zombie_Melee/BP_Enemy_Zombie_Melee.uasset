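; Melee zombie enemy character Blueprint that spawns its weapon on BeginPlay through the weapons manager component and signals when it is equipped.
; Attack and aggro alert events activate gameplay abilities by class, then fire their end callbacks on the next tick rather than waiting for ability completion.
; Overrides supply walk speeds per movement state and the ideal attack and defend ranges.
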(event EventBeginPlay
  (|CallParentFunction)
  (CallFunction|SpawnWeapon))

(event EventSpawnWeapon
  (Default|SpawnWeapon (Variables|Default|GetWeaponsManagerComponent) (Variables|Default|GetWeapon%20Class))
  (Variables|/Game/Weapons/WeaponsManagerComponent.WeaponsManagerComponent_C|GetEquippedWeapon (Variables|Default|GetWeaponsManagerComponent)
    (:then
      (Variables|Default|SetHasWeapon true)
      (Default|CallOnWeaponSpawn))
    (:else)))

(event EventAttack
  (Abilities|TryActivateAbilitybyClass (Variables|Default|GetGKAbilitySystemComponent) "/Game/EnemyCharacters/Enemies/Zombie_Melee/GA/GA_Zombie_Melee_Attack1.GA_Zombie_Melee_Attack1_C" true)
  (Utilities|FlowControl|DelayUntilNextTick)
  (Default|CallOnAttackEnd))

(event EventAggroAlert
  (Abilities|TryActivateAbilitybyClass (Variables|Default|GetGKAbilitySystemComponent) "/Game/EnemyCharacters/Enemies/Zombie_Melee/GA/GA_Zombie_AggroAlert.GA_Zombie_AggroAlert_C" true)
  (Utilities|FlowControl|DelayUntilNextTick)
  (Default|CallOnAggroAlertEnd))

(fn ConstructionScript
  (|CallParentFunction))

(fn SetMovementSpeed
  (params (Speed :type E_MovementSpeed%20Enum :default "NewEnumerator0"))
  (bind _output_get (Variables|/Script/Engine.CharacterMovementComponent|SetMaxWalkSpeed (Variables|Character|GetCharacterMovement) (Utilities|Select :Index Speed :NewEnumerator0 0.0 :NewEnumerator1 1e+02 :NewEnumerator2 3e+02 :NewEnumerator3 4e+02)))
  (return _output_get))

(fn GetIdealRange
  (return 1.5e+02 3.5e+02))
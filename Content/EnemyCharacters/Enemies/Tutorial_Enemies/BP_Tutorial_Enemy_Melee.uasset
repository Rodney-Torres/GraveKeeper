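; BP_Tutorial_Enemy_Melee is a tutorial melee zombie enemy that attacks and can spawn or delete its weapon.
; Attack activates the zombie melee gameplay ability and signals attack end on the next tick, without waiting for the ability to finish.
; Spawn and delete play scream montages whose notifies create or destroy the weapon through WeaponsManagerComponent and update HasWeapon.
; Each montage's completion calls the matching weapon spawn or delete callback.
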(event EventBeginPlay
  (|CallParentFunction) ; This node is disabled and will not be called.\nDrag off pins to build functionality.
)

(event EventSpawnWeapon
  (bind _notifyname (Animation|Montage|PlayMontage (Variables|Character|GetMesh) "/Game/EnemyCharacters/Enemies/Tutorial_Enemies/Montages/AM_Zombie_Scream_SpawnWeapon.AM_Zombie_Scream_SpawnWeapon")
    (:OnCompleted
      (Default|CallOnWeaponSpawn))
    (:OnNotifyBegin
      (switch name _notifyname
        (:SpawnWeapon
          (Default|SpawnWeapon (Variables|Default|GetWeaponsManagerComponent) (Variables|Default|GetWeapon%20Class))
          (Variables|/Game/Weapons/WeaponsManagerComponent.WeaponsManagerComponent_C|GetEquippedWeapon (Variables|Default|GetWeaponsManagerComponent)
            (:then
              (Variables|Default|SetHasWeapon true))
            (:else)))))))

(event EventDeleteWeapon
  (bind _notifyname (Animation|Montage|PlayMontage (Variables|Character|GetMesh) "/Game/EnemyCharacters/Enemies/Tutorial_Enemies/Montages/AM_Zombie_Scream_DeleteWeapon.AM_Zombie_Scream_DeleteWeapon")
    (:OnCompleted
      (Default|CallOnWeaponDelete))
    (:OnNotifyBegin
      (switch name _notifyname
        (:DeleteWeapon
          (Actor|DestroyActor (Variables|/Game/Weapons/WeaponsManagerComponent.WeaponsManagerComponent_C|GetEquippedWeapon (Variables|Default|GetWeaponsManagerComponent)))
          (Variables|Default|SetHasWeapon false))))))

(event Collision|EventActorBeginOverlap
  (params (OtherActor :type Actor%20Object%20Reference)))

(event EventTick
  (params (DeltaSeconds :type Float%20%28single-precision%29)))

(event EventAttack
  (Abilities|TryActivateAbilitybyClass (Variables|Default|GetGKAbilitySystemComponent) "/Game/EnemyCharacters/Enemies/Zombie_Melee/GA/GA_Zombie_Melee_Attack1.GA_Zombie_Melee_Attack1_C" true)
  (Utilities|FlowControl|DelayUntilNextTick)
  (Default|CallOnAttackEnd))

(fn ConstructionScript
  (|CallParentFunction))